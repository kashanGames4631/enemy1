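; BP_enemyG is an enemy character that roams between tagged actors and chases the player character when perceived.
; From BeginPlay it moves to a random tagged actor, pauses on arrival, then picks another.
; Any AI Perception update on BP_ThirdPersonCharacter raises walk speed and starts a move toward it, without checking whether sensing succeeded.
; When perception forgets that character, speed drops and the patrol loop resumes.
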(event OnTargetPerceptionUpdated(AIPerception)
  (params (Actor :type Actor%20Object%20Reference) (Stimulus :type AI%20Stimulus%20Structure))
  (bind _asbp_third_person_character (Utilities|Casting|CastToBP_ThirdPersonCharacter Actor))
  (Variables|/Script/Engine.CharacterMovementComponent|SetMaxWalkSpeed (Variables|Character|GetCharacterMovement) 5e+02)
  (AI|AIMoveTo self "0, 0, 0" _asbp_third_person_character 5.0 false))

(event OnTargetPerceptionForgotten(AIPerception)
  (params (Actor :type Actor%20Object%20Reference))
  (Utilities|Casting|CastToBP_ThirdPersonCharacter Actor)
  (Variables|/Script/Engine.CharacterMovementComponent|SetMaxWalkSpeed (Variables|Character|GetCharacterMovement) 3e+02)
  (bind _outactors (Actor|GetAllActorswithTag (Variables|Default|GetTag) :!label _label))
  (AI|AIMoveTo self "0, 0, 0" (.OutItem (Utilities|Array|Random _outactors)) 5.0 false
    (:OnSuccess
      (Utilities|FlowControl|Delay 2.0)
      (goto _label))))

(event EventBeginPlay
  (bind _outactors (Actor|GetAllActorswithTag (Variables|Default|GetTag) :!label _label))
  (AI|AIMoveTo self "0, 0, 0" (.OutItem (Utilities|Array|Random _outactors)) 5.0 false
    (:OnSuccess
      (Utilities|FlowControl|Delay 2.0)
      (goto _label))))

(event Collision|EventActorBeginOverlap
  (params (OtherActor :type Actor%20Object%20Reference)))

(event EventTick
  (params (DeltaSeconds :type Float%20%28single-precision%29)))

(fn ConstructionScript)